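; AudioManager is an actor Blueprint meant to play music tracks in sequence, chosen by a TrackNumber index.
; Tick runs TrackCheck every frame, which at track 0 plays Lonely_Troutman_II at the world origin and increments the index if the Audio component is not playing.
; The Portal branch compares constants and never runs.
; Main-menu logic for setting the starting track is present but unwired.
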(event EventBeginPlay)

(event EventTick
  (params (DeltaSeconds :type Float%20%28single-precision%29))
  (CallFunction|TrackCheck))

(fn ConstructionScript)

(fn TrackCheck
  (if (== 0 (Variables|Default|GetTrack%20Number))
    (Audio|PlaySoundatLocation "/Game/Audio/Music/Lonely_Troutman_II.Lonely_Troutman_II" "0, 0, 0")
    (if (not (Audio|Components|Audio|IsPlaying (Variables|Default|GetAudio)))
      (Variables|Default|SetTrack%20Number (+ (Variables|Default|GetTrack%20Number) 1)))
    (elif (== 0 1)
      (Audio|PlaySoundatLocation "/Game/Audio/Music/Portal.Portal" "0, 0, 0")
      (if (not (Audio|Components|Audio|IsPlaying (Variables|Default|GetAudio)))
        (Variables|Default|SetTrack%20Number (+ (Variables|Default|GetTrack%20Number) 1)))
      (elif true
        _))))