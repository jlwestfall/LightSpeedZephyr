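; LZ is a music controller Blueprint that plays the Portal sound at the world origin, scaled by a universal volume.
; BeginPlay resets the track index, and both it and Tick call TrackCheck.
; TrackCheck starts the sound while the index is zero, advancing it when the separate Audio component is not playing.
; The main-menu Play check and the second-track branch are disconnected, so neither runs.
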(event EventTick
  (params (DeltaSeconds :type Float%20%28single-precision%29))
  (CallFunction|TrackCheck))

(event EventBeginPlay
  (Variables|Default|SetTrack%20Number 0)
  (CallFunction|TrackCheck))

(fn ConstructionScript)

(fn TrackCheck
  (if (== 0 (Variables|Default|GetTrack%20Number))
    (Audio|PlaySoundatLocation "/Game/Audio/Music/Portal.Portal" "0, 0, 0" "0, 0, 0" (Variables|Default|GetUniveral%20Volume))
    (if (not (Audio|Components|Audio|IsPlaying (Variables|Default|GetAudio)))
      (Variables|Default|SetTrack%20Number (+ (Variables|Default|GetTrack%20Number) 1)))))